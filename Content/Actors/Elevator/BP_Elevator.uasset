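; Two-floor elevator actor that carries its cabin between floor heights when a button is pressed.
; BeginPlay spawns two floor buttons on mesh sockets and binds their press events, plus those of two referenced floor buttons, to MoveToFloor.
; MoveToFloor highlights the button, closes the sliding doors, moves the root to the target height, then resets the button and reopens the doors.
; Timed MoveComponentTo calls drive both cabin and doors.
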(event `self.ReceiveBeginPlay`
  (bind (_returnvalue_x _returnvalue_y _returnvalue_z) (`KismetMathLibrary.BreakVector` (`SceneComponent.K2_GetComponentLocation` (`self.DefaultSceneRoot`))))
  (bind _returnvalue (`|SpawnActorFromClass` "/Game/Actors/InteractiveActors/BP_ElevatorButton.BP_ElevatorButton_C" (`self.GetTransform`) "AlwaysSpawn" "OverrideRootScale" null null))
  (`self.K2_AttachToComponent` _returnvalue (`self.Mesh`) "FirstFloorButtonSocket" "SnapToTarget" "SnapToTarget" "SnapToTarget" true)
  (`/Game/Actors/InteractiveActors/BP_ElevatorButton.UpdateText` _returnvalue "1")
  (set `/Game/Actors/InteractiveActors/BP_ElevatorButton.FloorHeight` 0.0 _returnvalue)
  (add `/Game/Actors/InteractiveActors/BP_ElevatorButton.ElevatorButtonPressed` _returnvalue (delegate `ElevatorButtonPressed_Event_0`))
  (bind _returnvalue_2 (`|SpawnActorFromClass` "/Game/Actors/InteractiveActors/BP_ElevatorButton.BP_ElevatorButton_C" (`self.GetTransform`) "AlwaysSpawn" "OverrideRootScale" null null))
  (set `/Game/Actors/InteractiveActors/BP_ElevatorButton.FloorHeight` 300.0 _returnvalue_2)
  (`/Game/Actors/InteractiveActors/BP_ElevatorButton.UpdateText` _returnvalue_2 "2")
  (`self.K2_AttachToComponent` _returnvalue_2 (`self.Mesh`) "SecondFloorButtonSocket" "SnapToTarget" "SnapToTarget" "SnapToTarget" true)
  (add `/Game/Actors/InteractiveActors/BP_ElevatorButton.ElevatorButtonPressed` _returnvalue_2 (delegate `CustomEvent_0`))
  (add `/Game/Actors/InteractiveActors/BP_ElevatorButton.ElevatorButtonPressed` (`self.FirstFloorButton`) (delegate `ElevatorButtonPressed_Event_1`))
  (add `/Game/Actors/InteractiveActors/BP_ElevatorButton.ElevatorButtonPressed` (`self.SecondFloorButton`) (delegate `ElevatorButtonPressed_Event_2`))
  (set `self.CurrentFloorHeight` _returnvalue_z))

(event `ElevatorButtonPressed_Event_0`
  (params (FloorHeight :type "Float (double-precision)") (PressedButton :type "/Game/Actors/InteractiveActors/BP_ElevatorButton Object Reference"))
  (`self.MoveToFloor` FloorHeight PressedButton))

(event `CustomEvent_0`
  (params (FloorHeight :type "Float (double-precision)") (PressedButton :type "/Game/Actors/InteractiveActors/BP_ElevatorButton Object Reference"))
  (`self.MoveToFloor` FloorHeight PressedButton))

(event `ElevatorButtonPressed_Event_1`
  (params (FloorHeight :type "Float (double-precision)") (PressedButton :type "/Game/Actors/InteractiveActors/BP_ElevatorButton Object Reference"))
  (`self.MoveToFloor` FloorHeight PressedButton))

(event `ElevatorButtonPressed_Event_2`
  (params (FloorHeight :type "Float (double-precision)") (PressedButton :type "/Game/Actors/InteractiveActors/BP_ElevatorButton Object Reference"))
  (`self.MoveToFloor` FloorHeight PressedButton))

(event `MoveToFloor`
  (params (FloorHeight :type "Float (double-precision)") (PressedButton :type "/Game/Actors/InteractiveActors/BP_ElevatorButton Object Reference"))
  (bind _defaultsceneroot (`self.DefaultSceneRoot`))
  (bind (_relativelocation_x _relativelocation_y) (`KismetMathLibrary.BreakVector` (`SceneComponent.RelativeLocation` _defaultsceneroot)))
  (set `self.ElevatorMoving` true)
  (`/Engine/EditorBlueprintResources/StandardMacros.IsValid` PressedButton
    (:`Is Valid`
      (`/Game/Actors/InteractiveActors/BP_Button.ShowActiveColor` PressedButton))
    (:`Is Not Valid`
      _))
  (if (not (`self.DoorsClosed`))
    (`self.CloseDoors`)
    (`KismetSystemLibrary.Delay` (`self.DoorsMovingTime`)))
  (if (not (== FloorHeight (`self.CurrentFloorHeight`)))
    (`KismetSystemLibrary.MoveComponentTo` _defaultsceneroot (`KismetMathLibrary.MakeVector` _relativelocation_x _relativelocation_y FloorHeight) (`SceneComponent.RelativeRotation` _defaultsceneroot) false false 3.0)
    (set `self.CurrentFloorHeight` FloorHeight))
  (`/Engine/EditorBlueprintResources/StandardMacros.IsValid` PressedButton
    (:`Is Valid`
      (`/Game/Actors/InteractiveActors/BP_Button.ShowDefaultColor` PressedButton)
      (`/Game/Actors/InteractiveActors/BP_Button.ReleaseButton` PressedButton))
    (:`Is Not Valid`
      _))
  (`self.OpenDoors`)
  (set `self.ElevatorMoving` false))

(event `CloseDoors`
  (bind _doorleft (`self.DoorLeft`))
  (bind _doorright (`self.DoorRight`))
  (`|ExecutionSequence`
    (:`then_0`
      (`KismetSystemLibrary.MoveComponentTo` _doorright (+ (`SceneComponent.RelativeLocation` _doorright) (-95.0 0.0 0.0)) (`SceneComponent.RelativeRotation` _doorright) false false (`self.DoorsMovingTime`)))
    (:`then_1`
      (`KismetSystemLibrary.MoveComponentTo` _doorleft (+ (`SceneComponent.RelativeLocation` _doorleft) (95.0 0.0 -0.0)) (`SceneComponent.RelativeRotation` _doorleft) false false (`self.DoorsMovingTime`))
      (set `self.DoorsClosed` true))))

(event `OpenDoors`
  (bind _doorright (`self.DoorRight`))
  (bind _doorleft (`self.DoorLeft`))
  (`|ExecutionSequence`
    (:`then_0`
      (`KismetSystemLibrary.MoveComponentTo` _doorright (+ (`SceneComponent.RelativeLocation` _doorright) (95.0 0.0 0.0)) (`SceneComponent.RelativeRotation` _doorright) false false (`self.DoorsMovingTime`)))
    (:`then_1`
      (`KismetSystemLibrary.MoveComponentTo` _doorleft (+ (`SceneComponent.RelativeLocation` _doorleft) (-95.0 0.0 0.0)) (`SceneComponent.RelativeRotation` _doorleft) false false (`self.DoorsMovingTime`))
      (set `self.DoorsClosed` false))))

(fn `UserConstructionScript`)