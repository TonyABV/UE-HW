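; Door actor that swings open when its linked buttons are pressed in the order given by a code string.
; On BeginPlay it binds each button's press event, then compares the incoming button ID to the code's current digit, debug-printing the expected one.
; A match advances the index and the final match rotates the door 90 degrees in yaw.
; A mismatch releases the buttons and resets progress.
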(event `self.ReceiveBeginPlay`
  (for _array_element (`self.Buttons`)
    (add `/Game/Actors/InteractiveActors/BP_Button.OnButtonPressed` _array_element (delegate `OnButtonPressed_Event_0`))))

(event `OnButtonPressed_Event_0`
  (params (ButtonID :type Integer))
  (`self.TryOpen` ButtonID))

(event `AbortProgress`
  (for _array_element (`self.Buttons`)
    (`/Game/Actors/InteractiveActors/BP_Button.ReleaseButton` _array_element)
    (set `self.CurrentSign` 0)))

(event `OpenDoor`
  (bind _door (`self.Door`))
  (bind (_relativerotation_roll _relativerotation_pitch _relativerotation_yaw) (`KismetMathLibrary.BreakRotator` (`SceneComponent.RelativeRotation` _door)))
  (`SceneComponent.SetMobility` (`self.Door`) "Movable")
  (`KismetSystemLibrary.MoveComponentTo` _door (`SceneComponent.RelativeLocation` _door) (`KismetMathLibrary.MakeRotator` _relativerotation_roll _relativerotation_pitch (+ _relativerotation_yaw 90.0)) false false 1.0))

(fn `UserConstructionScript`)