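; BP_Catapult is a physics-driven catapult actor operated by its CatapultLever.
; The lever's max-angle event calls Reload at the positive limit and Fire at the negative one.
; Fire powers the physics constraint's angular drive; Reload zeroes it, waits briefly, then spawns a projectile at the spawn point.
; An automatic fire-and-reload loop is left unconnected and never runs.
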(event `self.ReceiveBeginPlay`
  (add `/Game/Actors/InteractiveActors/BP_LeverActor.MaxAngleReached` (`self.CatapultLever`) (delegate `MaxAngleReached_Event_0`)))

(event `MaxAngleReached_Event_0`
  (params (PositiveAngle :type Boolean))
  (if PositiveAngle
    (`self.Reload`)
    (else
      (`self.Fire`))))

(fn `UserConstructionScript`)