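; Interactive lever actor that pivots while its grab sphere is held and signals when it reaches either angle limit.
; While grabbed, Tick calls RotateLever, which adds the world X offset between Arrow and Sphere to the pitch, clamped to MaxAngles.
; DoOnce gates fire MaxAngleReached once per arrival, with a boolean identifying the limit.
; On release, the lever optionally eases back to its BeginPlay transform.
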(event `self.ReceiveBeginPlay`
  (bind _lever (`self.Lever`))
  (set `self.DefaultRelative Location` (`SceneComponent.RelativeLocation` _lever))
  (set `self.DefaultRotation` (`SceneComponent.RelativeRotation` _lever)))

(event `self.ReceiveTick`
  (params (DeltaSeconds :type "Float (single-precision)"))
  (if (`self.SphereGrabbed`)
    (`self.RotateLever`
      (:`NewParam`
        (goto _label :!via `Reset`)))
    (elif (`self.AutoReturnToDefault`)
      (`/Engine/EditorBlueprintResources/StandardMacros.DoOnce` false :!label _label
        (:`Completed`
          (`KismetSystemLibrary.MoveComponentTo` (`self.Lever`) (`self.DefaultRelative Location`) (`self.DefaultRotation`) false false 1.0))))))

(event `self.SphereGrab.OnGrabbed`
  (set `self.SphereGrabbed` true))

(event `self.SphereGrab.OnDropped`
  (set `self.SphereGrabbed` false))

(fn `UserConstructionScript`)