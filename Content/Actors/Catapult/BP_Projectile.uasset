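; Catapult projectile actor that deals area damage and drives a radial force when it hits something.
; When its Sphere overlaps an actor other than itself or its owner, it applies radial damage centered on that actor's location.
; It then sets the RadialForce component's radius and strength, sharing the damage radius, and shortens its lifespan so it disappears a moment later.
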(event `self.ReceiveBeginPlay`)

(event `self.StaticMesh.OnComponentBeginOverlap`
  (params (OverlappedComponent :type "PrimitiveComponent Object Reference") (OtherActor :type "Actor Object Reference") (OtherComp :type "PrimitiveComponent Object Reference") (OtherBodyIndex :type Integer) (bFromSweep :type Boolean) (SweepResult :type "HitResult Structure (by ref)")))

(event `self.Sphere.OnComponentBeginOverlap`
  (params (OverlappedComponent :type "PrimitiveComponent Object Reference") (OtherActor :type "Actor Object Reference") (OtherComp :type "PrimitiveComponent Object Reference") (OtherBodyIndex :type Integer) (bFromSweep :type Boolean) (SweepResult :type "HitResult Structure (by ref)"))
  (bind _radialforce (`self.RadialForce`))
  (if (and (!= OtherActor (`self.GetOwner`)) (!= OtherActor self))
    (`GameplayStatics.ApplyRadialDamage` :`BaseDamage` (`self.Damage`) :`Origin` (`self.K2_GetActorLocation` OtherActor) :`DamageRadius` (`self.Radius`) :`DamageCauser` null :`InstigatedByController` null)
    (set `RadialForceComponent.Radius` (`self.Radius`) _radialforce)
    (set `RadialForceComponent.ForceStrength` (`self.Strenght`) _radialforce)
    (`self.SetLifeSpan` 0.1)))

(fn `UserConstructionScript`)