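; BP_ButtonComponent is a pressable VR button component that reacts to overlaps from components attached to a motion controller.
; A press slides it along relative Y over a short latent move, then fires OnButtonPressed and optionally auto-returns.
; ButtonPressed blocks retriggering until release completes.
; A dynamic material instance starts at the default color and exposes events to switch between active and default colors.
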(event `self.ReceiveBeginPlay`
  (bind _returnvalue (`self.CreateDynamicMaterialInstance` 0 (`self.GetMaterial` 0)))
  (set `self.DynamicButtonMaterial` _returnvalue)
  (add `self.OnComponentBeginOverlap` (delegate `OnComponentBeginOverlap_Event_0`))
  (`self.ShowDefaultColor`))

(event `OnComponentBeginOverlap_Event_0` :!signature `self.OnComponentBeginOverlap`
  (params (OverlappedComponent :type "PrimitiveComponent Object Reference") (OtherActor :type "Actor Object Reference") (OtherComp :type "PrimitiveComponent Object Reference") (OtherBodyIndex :type Integer) (bFromSweep :type Boolean) (SweepResult :type "HitResult Structure (by ref)"))
  (bind _returnvalue (`self.GetAttachParent` OtherComp))
  (if (not (`self.ButtonPressed`))
    (`/Engine/EditorBlueprintResources/StandardMacros.IsValid` _returnvalue
      (:`Is Valid`
        (cast `MotionControllerComponent` _returnvalue)
        (`self.PressButton`)))))

(event `PressButton`
  (set `self.ButtonPressed` true)
  (`KismetSystemLibrary.MoveComponentTo` self (+ (`self.RelativeLocation`) (`KismetMathLibrary.MakeVector` 0.0 (* -1 (`self.Amplitude`)))) (`self.RelativeRotation`) false false 0.3)
  (`self.OnButtonPressed`)
  (if (`self.EnableAutoReturn`)
    (`self.ReleaseButton`)))

(event `ReleaseButton`
  (`KismetSystemLibrary.MoveComponentTo` self (+ (`KismetMathLibrary.MakeVector` 0.0 (`self.Amplitude`)) (`self.RelativeLocation`)) (`self.RelativeRotation`) false false 0.3)
  (set `self.ButtonPressed` false))

(event `ShowActiveColor`
  (`MaterialInstanceDynamic.SetVectorParameterValue` (`self.DynamicButtonMaterial`) "Color" (`self.ActiveColor`)))

(event `ShowDefaultColor`
  (`MaterialInstanceDynamic.SetVectorParameterValue` (`self.DynamicButtonMaterial`) "Color" (`self.DefaultColor`)))