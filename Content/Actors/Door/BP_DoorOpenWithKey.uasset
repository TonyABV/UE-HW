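; Door actor that swings open when its matching key actor overlaps its trigger box.
; The overlap destroys that actor, then MoveKey reveals the hidden key and slides it over one second before OpenDoor yaws the door 90 degrees via MoveComponentTo.
; TryOpen and Check sketch a digit-by-digit code check on empty strings, with no caller in this graph.
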(event `self.ReceiveBeginPlay`
  (`SceneComponent.SetVisibility` (`self.Key_`) false false))

(event `OpenDoor`
  (bind _door (`self.Door`))
  (bind (_relativerotation_roll _relativerotation_pitch _relativerotation_yaw) (`KismetMathLibrary.BreakRotator` (`SceneComponent.RelativeRotation` _door)))
  (`SceneComponent.SetMobility` (`self.Door`) "Movable")
  (`KismetSystemLibrary.MoveComponentTo` _door (`SceneComponent.RelativeLocation` _door) (`KismetMathLibrary.MakeRotator` _relativerotation_roll _relativerotation_pitch (+ _relativerotation_yaw 90.0)) false false 1.0))

(event `self.Box.OnComponentBeginOverlap`
  (params (OverlappedComponent :type "PrimitiveComponent Object Reference") (OtherActor :type "Actor Object Reference") (OtherComp :type "PrimitiveComponent Object Reference") (OtherBodyIndex :type Integer) (bFromSweep :type Boolean) (SweepResult :type "HitResult Structure (by ref)"))
  (if (== OtherActor (`self.Key`))
    (`self.K2_DestroyActor` (`self.Key`))
    (`self.MoveKey`
      (:`Completed`
        (`self.OpenDoor`)))))

(fn `UserConstructionScript`)