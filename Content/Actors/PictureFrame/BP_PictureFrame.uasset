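; BP_PictureFrame is a picture frame actor that shows whether a designated TargetActor is inside its box volume.
; Box begin and end overlap events set or clear the TargetInBox flag, ignoring any other actor.
; Tick reads that flag every frame and sets the Plane's material to SuccessMat or BaseMat, rather than swapping it only when the overlap changes.
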(event `self.ReceiveTick`
  (params (DeltaSeconds :type "Float (single-precision)"))
  (bind _plane (`self.Plane`))
  (if (`self.TargetInBox`)
    (`PrimitiveComponent.SetMaterial` _plane 0 (`self.SuccessMat`))
    (else
      (`PrimitiveComponent.SetMaterial` _plane 0 (`self.BaseMat`)))))

(event `self.Box.OnComponentBeginOverlap`
  (params (OverlappedComponent :type "PrimitiveComponent Object Reference") (OtherActor :type "Actor Object Reference") (OtherComp :type "PrimitiveComponent Object Reference") (OtherBodyIndex :type Integer) (bFromSweep :type Boolean) (SweepResult :type "HitResult Structure (by ref)"))
  (if (== OtherActor (`self.TargetActor`))
    (set `self.TargetInBox` true)))

(event `self.Box.OnComponentEndOverlap`
  (params (OverlappedComponent :type "PrimitiveComponent Object Reference") (OtherActor :type "Actor Object Reference") (OtherComp :type "PrimitiveComponent Object Reference") (OtherBodyIndex :type Integer))
  (if (== OtherActor (`self.TargetActor`))
    (set `self.TargetInBox` false)))

(fn `UserConstructionScript`)