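; BP_DoorClosable is a door actor that its handle switches between open and closed states.
; On BeginPlay it spawns a BP_DoorHandle on the door mesh's HandleSocket, binds its MaxAngleReached event and applies the initial state.
; A positive max angle sets closed, otherwise open.
; Open enables physics simulation on the door, closed disables it, and both text renders update to match.
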(event `self.ReceiveBeginPlay`
  (bind _returnvalue (`|SpawnActorFromClass` "/Game/Actors/Door/BP_DoorHandle.BP_DoorHandle_C" (`self.GetTransform`) "AlwaysSpawn" "OverrideRootScale" null null))
  (`self.K2_AttachToComponent` _returnvalue (`self.Door`) "HandleSocket" "SnapToTarget" "SnapToTarget" "SnapToTarget" false)
  (add `/Game/Actors/Door/BP_DoorHandle.MaxAngleReached` _returnvalue (delegate `MaxAngleReached_Event_0`))
  (`self.Open/Close Door`))

(event `MaxAngleReached_Event_0`
  (params (PositiveAngle :type Boolean))
  (set `self.DoorOpend` (not PositiveAngle))
  (`self.Open/Close Door`))

(fn `UserConstructionScript`)