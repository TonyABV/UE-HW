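; BP_DoorOpenWithLever is a door actor that toggles open and closed when its lever reaches its positive maximum angle.
; The lever's delegate, bound on BeginPlay, picks OpenDoor or CloseDoor from a state flag, each using MoveComponentTo to roll the door a quarter turn over one second.
; Separate Check and TryOpen graphs sketch a digit-sequence unlock, but their source strings are empty and the lever logic never calls them.
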(event `self.ReceiveBeginPlay`
  (add `/Game/Actors/InteractiveActors/BP_LeverActor.MaxAngleReached` (`self.Lever`) (delegate `MaxAngleReached_Event_0`)))

(event `MaxAngleReached_Event_0`
  (params (PositiveAngle :type Boolean))
  (if PositiveAngle
    (if (`self.DoorOpend`)
      (`self.CloseDoor`)
      (else
        (`self.OpenDoor`)))))

(event `OpenDoor`
  (bind _door (`self.Door`))
  (bind (_relativerotation_roll _relativerotation_pitch _relativerotation_yaw) (`KismetMathLibrary.BreakRotator` (`SceneComponent.RelativeRotation` _door)))
  (`SceneComponent.SetMobility` (`self.Door`) "Movable")
  (`KismetSystemLibrary.MoveComponentTo` _door (`SceneComponent.RelativeLocation` _door) (`KismetMathLibrary.MakeRotator` (+ _relativerotation_roll 90.0) _relativerotation_pitch _relativerotation_yaw) false false 1.0)
  (set `self.DoorOpend` true))

(event `CloseDoor`
  (bind _door (`self.Door`))
  (bind (_relativerotation_roll _relativerotation_pitch _relativerotation_yaw) (`KismetMathLibrary.BreakRotator` (`SceneComponent.RelativeRotation` _door)))
  (`SceneComponent.SetMobility` (`self.Door`) "Movable")
  (`KismetSystemLibrary.MoveComponentTo` _door (`SceneComponent.RelativeLocation` _door) (`KismetMathLibrary.MakeRotator` (+ _relativerotation_roll -90.0) _relativerotation_pitch _relativerotation_yaw) false false 1.0)
  (set `self.DoorOpend` false))

(fn `UserConstructionScript`)