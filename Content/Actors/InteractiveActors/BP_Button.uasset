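; BP_Button is an interactive VR push button actor that is pressed by touch from a component attached to a motion controller.
; An overlap while unpressed latches the pressed state, moves the button component down and calls OnButtonPressed.
; ReleaseButton, not triggered within this graph, raises it again, clears the state and calls OnButtonReleased.
; Separate events switch between active and default colors through a dynamic material created at BeginPlay.
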(event `self.ReceiveBeginPlay`
  (bind _button (`self.Button`))
  (bind _returnvalue (`PrimitiveComponent.CreateDynamicMaterialInstance` _button 0 (`PrimitiveComponent.GetMaterial` _button 0) "None"))
  (set `self.DynamicButtonMaterial` _returnvalue))

(event `self.Button.OnComponentBeginOverlap`
  (params (OverlappedComponent :type "PrimitiveComponent Object Reference") (OtherActor :type "Actor Object Reference") (OtherComp :type "PrimitiveComponent Object Reference") (OtherBodyIndex :type Integer) (bFromSweep :type Boolean) (SweepResult :type "HitResult Structure (by ref)"))
  (bind _returnvalue (`SceneComponent.GetAttachParent` OtherComp))
  (if (not (`self.ButtonPressed`))
    (`/Engine/EditorBlueprintResources/StandardMacros.IsValid` _returnvalue
      (:`Is Valid`
        (cast `MotionControllerComponent` _returnvalue)
        (`self.PressButton`)))))

(event `PressButton`
  (bind _button (`self.Button`))
  (set `self.ButtonPressed` true)
  (`KismetSystemLibrary.MoveComponentTo` _button (+ (`SceneComponent.RelativeLocation` _button) (0.0 0.0 -5.0)) (`SceneComponent.RelativeRotation` _button))
  (`self.OnButtonPressed`))

(event `ReleaseButton`
  (bind _button (`self.Button`))
  (`KismetSystemLibrary.MoveComponentTo` _button (+ (0.0 0.0 5.0) (`SceneComponent.RelativeLocation` _button)) (`SceneComponent.RelativeRotation` _button))
  (set `self.ButtonPressed` false)
  (`self.OnButtonReleased`))

(event `ShowActiveColor`
  (`MaterialInstanceDynamic.SetVectorParameterValue` (`self.DynamicButtonMaterial`) "Color" (`self.ActiveColor`)))

(event `ShowDefaultColor`
  (`MaterialInstanceDynamic.SetVectorParameterValue` (`self.DynamicButtonMaterial`) "Color" (`self.DefaultColor`)))

(fn `UserConstructionScript`)