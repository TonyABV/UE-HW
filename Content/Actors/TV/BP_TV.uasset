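; BP_TV is a television actor controlled through a referenced RemoteController's on/off and switch-channel dispatchers, bound at BeginPlay.
; A dynamic material on the screen Plane shows OffColor when off, or the current entry of the Channels color array when on.
; Switching works only while on and wraps around in both directions.
; A TextRender displays the one-based channel number and is hidden when the TV is turned off.
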(event `self.ReceiveBeginPlay`
  (bind _plane (`self.Plane`))
  (bind _remotecontroller (`self.RemoteController`))
  (bind _returnvalue (`PrimitiveComponent.CreateDynamicMaterialInstance` _plane 0 (`PrimitiveComponent.GetMaterial` _plane 0) "None"))
  (set `self.DynamicMat` _returnvalue)
  (`MaterialInstanceDynamic.SetVectorParameterValue` _returnvalue "Color" (`self.OffColor`))
  (add `/Game/Actors/TV/BP_RemoteController.On/Off Pressed` _remotecontroller (delegate `On/Off Pressed_Event_0`))
  (add `/Game/Actors/TV/BP_RemoteController.SwitchChannel` _remotecontroller (delegate `SwitchChannel_Event_0`)))

(event `SwitchChannel_Event_0`
  (params (SwitchForward :type Boolean))
  (`self.SwitchChannel` SwitchForward))

(event `On/Off Pressed_Event_0`
  (`self.Turn on/off`))

(event `Turn on/off`
  (bind _textrender (`self.TextRender`))
  (if (`self.On/Off`)
    (`MaterialInstanceDynamic.SetVectorParameterValue` (`self.DynamicMat`) "Color" (`self.OffColor`))
    (`SceneComponent.SetVisibility` (`self.TextRender`) false false)
    (set `self.On/Off` false)
    (else
      (`MaterialInstanceDynamic.SetVectorParameterValue` (`self.DynamicMat`) "Color" (`|GetArrayItem` (`self.Channels`) (`self.CurrentChannel`)))
      (`TextRenderComponent.K2_SetText` _textrender (`KismetTextLibrary.Conv_IntToText` (+ (`self.CurrentChannel`) 1)))
      (`SceneComponent.SetVisibility` _textrender true false)
      (set `self.On/Off` true))))

(event `SwitchChannel`
  (params (SwitchForward :type Boolean))
  (bind _channels (`self.Channels`))
  (bind _currentchannel (`self.CurrentChannel`))
  (bind _dynamicmat (`self.DynamicMat`))
  (if (`self.On/Off`)
    (if SwitchForward
      (bind _output_get (set `self.CurrentChannel` (mod (+ (`self.CurrentChannel`) 1) (`KismetArrayLibrary.Array_Length` (`self.Channels`)))))
      (`MaterialInstanceDynamic.SetVectorParameterValue` _dynamicmat "Color" (`|GetArrayItem` _channels _output_get))
      (else
        (if (== _currentchannel 0)
          (set `self.CurrentChannel` (- (`KismetArrayLibrary.Array_Length` (`self.Channels`)) 1))
          (else
            (set `self.CurrentChannel` (- _currentchannel 1))))
        (`MaterialInstanceDynamic.SetVectorParameterValue` _dynamicmat "Color" (`|GetArrayItem` _channels (`self.CurrentChannel`)))))
    (`TextRenderComponent.K2_SetText` (`self.TextRender`) (`KismetTextLibrary.Conv_IntToText` (+ (`self.CurrentChannel`) 1)))))

(fn `UserConstructionScript`)