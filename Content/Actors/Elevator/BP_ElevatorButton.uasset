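; Elevator button actor that shows a floor label and announces which floor height was requested when pressed.
; On begin play it binds to its OnButtonPressed dispatcher and sets the Level text from LevelText.
; A press is re-broadcast through the ElevatorButtonPressed dispatcher with FloorHeight and a reference to the button.
; An UpdateText event lets the label change at runtime.
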(event `self.ReceiveBeginPlay`
  (`parent.ReceiveBeginPlay`)
  (add `self.OnButtonPressed` (delegate `OnButtonPressed_Event_0`))
  (`TextRenderComponent.K2_SetText` (`self.Level`) (`self.LevelText`)))

(event `OnButtonPressed_Event_0`
  (`self.ElevatorButtonPressed` (`self.FloorHeight`) self))

(event `UpdateText`
  (params (Text :type Text))
  (`TextRenderComponent.K2_SetText` (`self.Level`) Text))

(fn `UserConstructionScript`
  (`parent.UserConstructionScript`))