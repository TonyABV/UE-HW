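; BP_MovableWall is a wall actor that slides open once every BP_PictureFrame in the level reports its target in box.
; Each Tick it gathers all picture frames and checks TargetInBox, breaking at the first unsatisfied one.
; When all pass, a DoOnce fires Move, which makes the mesh movable and interpolates it by AdditionalLocation over a second.
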(event `self.ReceiveBeginPlay`)

(event `self.ReceiveTick`
  (params (DeltaSeconds :type "Float (single-precision)"))
  (bind _outactors (`GameplayStatics.GetAllActorsOfClass` "/Game/Actors/PictureFrame/BP_PictureFrame.BP_PictureFrame_C"))
  (for _array_element _outactors
    (if (`/Game/Actors/PictureFrame/BP_PictureFrame.TargetInBox` _array_element)
      (set `self.CanOpen` true)
      (else
        (set `self.CanOpen` false)
        (break))))
  (if (`self.CanOpen`)
    (`/Engine/EditorBlueprintResources/StandardMacros.DoOnce` false
      (:`Completed`
        (`self.Move`)))))

(event `Move`
  (bind _staticmesh (`self.StaticMesh`))
  (`SceneComponent.SetMobility` _staticmesh "Movable")
  (`KismetSystemLibrary.MoveComponentTo` _staticmesh (+ (`SceneComponent.RelativeLocation` _staticmesh) (`self.AdditionalLocation`)) (`SceneComponent.K2_GetComponentRotation` _staticmesh) false false 1.0))

(fn `UserConstructionScript`)