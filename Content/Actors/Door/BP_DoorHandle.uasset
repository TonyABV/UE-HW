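; Door handle actor with two grabbable spheres that turn the handle within angle limits.
; While a sphere is grabbed, Tick calls RotateHandle, adding the world Y offset between Arrow and that sphere to the clamped pitch.
; RotateHandle calls MaxAngleReached once upon reaching either limit, with a flag indicating which.
; With AutoReturnToDefault enabled, a released handle moves back to its transform cached at BeginPlay.
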(event `self.ReceiveBeginPlay`
  (bind _handle (`self.Handle`))
  (set `self.DefaultRelative Location` (`SceneComponent.RelativeLocation` _handle))
  (set `self.DefaultRotation` (`SceneComponent.RelativeRotation` _handle)))

(event `self.ReceiveTick`
  (params (DeltaSeconds :type "Float (single-precision)"))
  (if (`self.Sphere_1Grabbed`)
    (`self.RotateHandle` (`self.Sphere 1`)
      (:`NewParam`
        (goto _label :!via `Reset`)))
    (elif (`self.Sphere_2Grabbed`)
      (`self.RotateHandle` (`self.Sphere 2`)
        (:`NewParam`
          (goto _label :!via `Reset`)))
      (elif (`self.AutoReturnToDefault`)
        (`/Engine/EditorBlueprintResources/StandardMacros.DoOnce` false :!label _label
          (:`Completed`
            (`KismetSystemLibrary.MoveComponentTo` (`self.Handle`) (`self.DefaultRelative Location`) (`self.DefaultRotation`) false false 1.0)))))))

(event `self.Sphere 1 Grab.OnGrabbed`
  (set `self.Sphere_1Grabbed` true))

(event `self.Sphere 1 Grab.OnDropped`
  (set `self.Sphere_1Grabbed` false))

(event `self.Sphere 2 Grab.OnGrabbed`
  (set `self.Sphere_2Grabbed` true))

(event `self.Sphere 2 Grab.OnDropped`
  (set `self.Sphere_2Grabbed` false))

(fn `UserConstructionScript`)